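; Treasure actor that registers its string with the player's Performer character when any actor overlaps it.
; On BeginPlay it caches the player as a Performer and binds a custom event to that character's EnableTreasureChestAction dispatcher.
; When the event fires, a TreasureString equality check gates a debug print of the string, with no other chest action implemented.
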(event Custom|CustomEvent
  (params (TreasureString :type String) (TreasureAbility :type EPlayerTreasureAction%20Enum :default "IncludeTreasure") (AllGood :type Boolean))
  (if (Utilities|Enum|Equal(Enum) TreasureString (Variables|Default|GetTreasureString))
    (if true
      (Development|PrintString TreasureString)
      (else
        (Development|PrintString TreasureString)))))

(event EventBeginPlay
  (bind _asperformer (Utilities|Casting|CastToPerformer (Game|GetPlayerCharacter 0)))
  (bind _output_get (Variables|Default|SetPerformer _asperformer))
  (EventDispatchers|BindEventtoEnableTreasureChestAction _output_get (delegate Custom|CustomEvent)))

(event Collision|EventActorBeginOverlap
  (params (OtherActor :type Actor%20Object%20Reference))
  (Class|Performer|IncludeTreasure (Variables|Default|GetPerformer) (Variables|Default|GetTreasureString)))

(fn ConstructionScript)